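; Laser shooter Blueprint for the shield demo that periodically fires lasers at the player while within range.
; BeginPlay finds the target by the PlayerShield tag and randomizes the starting timer to stagger shots.
; Tick checks distance and advances the timer, calling ShootLaser to spawn a laser set up with the shooter root and target.
; EndPlay destroys the most recently spawned laser.
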(event EventBeginPlay
  (bind _outactors (Actor|GetAllActorswithTag "PlayerShield"))
  (for _array_element _outactors
    (Variables|Default|SetplayerAref _array_element)
    (Variables|Default|SetlaserSpawnTimer (* (Variables|Default|GetlaserSpawnRate) (Math|Random|RandomFloat)))))

(event Collision|EventActorBeginOverlap
  (params (OtherActor :type Actor%20Object%20Reference)))

(event EventTick
  (params (DeltaSeconds :type Float%20%28single-precision%29))
  (if (< (Math|Vector|Distance(Vector) (Transformation|GetWorldLocation (Variables|Default|GetDefaultSceneRoot)) (Transformation|GetWorldLocation (Variables|/Script/Engine.Actor|GetRootComponent (Variables|Default|GetplayerAref)))) (Variables|Default|GetshootRange))
    ;[1 1 1] Count down bullet spawning timer
    (bind _output_get (Variables|Default|SetlaserSpawnTimer (+ DeltaSeconds (Variables|Default|GetlaserSpawnTimer))))
    (if (> _output_get (Variables|Default|GetlaserSpawnRate))
      (CallFunction|ShootLaser))))

(event EventEndPlay
  (params (EndPlayReason :type EEndPlayReason%20Enum :default "Destroyed"))
  (bind _mylaserref (Variables|Default|GetmyLaserRef))
  (Utilities|IsValid _mylaserref
    (:Is%20Valid
      (Actor|DestroyActor _mylaserref))))

(fn ConstructionScript)

(fn ShootLaser
  (Variables|Default|SetlaserSpawnTimer 0.0)
  (bind _returnvalue (Game|SpawnActorfromClass "/Game/Shield_demo/Laser_Blueprint.Laser_Blueprint_C" (Transformation|GetWorldTransform (Variables|Default|GetDefaultSceneRoot)) "Undefined" 0 0))
  (Default|SetupLaser _returnvalue (Variables|Default|GetDefaultSceneRoot) (Variables|Default|GetplayerAref))
  (Variables|Default|SetmyLaserRef _returnvalue))