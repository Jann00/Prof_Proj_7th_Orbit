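; BlockWallBP is a group of BlockEnemyTemp drones, held as child actors under a Sphere component, that flies in along a spline.
; While FlyingIn is true, Tick advances the Sphere along FlyInSpline at FlyInSpeed.
; It orients the Sphere using a short look-ahead on the spline with fixed angle offsets.
; Near the spline's end, it stops the flight and makes each enemy's Shield visible.
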(event EventBeginPlay)

(event Collision|EventActorBeginOverlap
  (params (OtherActor :type Actor%20Object%20Reference)))

(event EventTick
  (params (DeltaSeconds :type Float%20%28single-precision%29))
  (if (Variables|Default|GetFlyingIn)
    (CallFunction|MoveDownSpline)))

(fn ConstructionScript)

(fn MoveDownSpline
  (bind _flyinspline (Variables|Default|GetFlyInSpline))
  (Transformation|SetWorldLocation (Variables|Default|GetSphere) (Spline|GetLocationatDistanceAlongSpline (Variables|Default|GetFlyInSpline) (Variables|Default|GetFlightPathProgress) "World") false false)
  (if (< (Variables|Default|GetFlightPathProgress) (Spline|GetSplineLength (Variables|Default|GetFlyInSpline)))
    (Variables|Default|SetFlightPathProgress (+ (Variables|Default|GetFlightPathProgress) (* (Utilities|Time|GetWorldDeltaSeconds) (Variables|Default|GetFlyInSpeed))))
    (if (< (+ (Variables|Default|GetFlightPathProgress) 1.1) (Spline|GetSplineLength (Variables|Default|GetFlyInSpline)))
      (Transformation|SetWorldRotation (Variables|Default|GetSphere) (Math|Rotator|MakeRotator (+ (.Roll (Math|Rotator|BreakRotator (Math|Conversions|RotationFromXVector (- (Spline|GetLocationatDistanceAlongSpline _flyinspline (+ (Variables|Default|GetFlightPathProgress) 1.0) "World") (Spline|GetLocationatDistanceAlongSpline _flyinspline (Variables|Default|GetFlightPathProgress) "World"))))) 9e+01) (+ (.Pitch (Math|Rotator|BreakRotator (Math|Conversions|RotationFromXVector (- (Spline|GetLocationatDistanceAlongSpline _flyinspline (+ (Variables|Default|GetFlightPathProgress) 1.0) "World") (Spline|GetLocationatDistanceAlongSpline _flyinspline (Variables|Default|GetFlightPathProgress) "World"))))) -9e+01) (.Yaw (Math|Rotator|BreakRotator (Math|Conversions|RotationFromXVector (- (Spline|GetLocationatDistanceAlongSpline _flyinspline (+ (Variables|Default|GetFlightPathProgress) 1.0) "World") (Spline|GetLocationatDistanceAlongSpline _flyinspline (Variables|Default|GetFlightPathProgress) "World")))))) false false)
      (else
        (Variables|Default|SetFlyingIn false)
        (for _array_element (Components|GetChildrenComponents (Variables|Default|GetSphere) true)
          (bind _aschild_actor_component (Utilities|Casting|CastToChildActorComponent _array_element))
          (bind _asblock_enemy_temp (Utilities|Casting|CastToBlockEnemyTemp (Variables|/Script/Engine.ChildActorComponent|GetChildActor _aschild_actor_component)))
          (Rendering|SetVisibility (Variables|/Game/Shield_demo/Enemies/BlockEnemyTemp.BlockEnemyTemp_C|GetShield _asblock_enemy_temp) true false))))))