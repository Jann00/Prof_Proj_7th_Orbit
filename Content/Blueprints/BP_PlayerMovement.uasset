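; Player movement Blueprint that flies the player forward along its facing each tick, pausing while turning.
; Camera joystick input offsets the player child within the forward path, either freely within clamps or following the stick inside a radius.
; Boosting burns fuel from a fuel manager, then eases max speed back to default.
; Wall hits halve speed, shake the camera, rumble and end boost, while steam overlaps blur the camera.
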(event OnComponentBeginOverlap(Box)
  (params (OverlappedComponent :type Primitive%20Component%20Object%20Reference) (OtherActor :type Actor%20Object%20Reference) (OtherComp :type Primitive%20Component%20Object%20Reference) (OtherBodyIndex :type Integer) (bFromSweep :type Boolean) (SweepResult :type Hit%20Result%20Structure%20%28by%20ref%29))
  (bind _self self)
  (bind _camera (Variables|Default|GetCamera))
  ;[1 1 1] Wall collision
  (if (not (Variables|/Game/Blueprints/BP_PlayerCamera.BP_PlayerCamera_C|GetShaking (Variables|Default|GetCamera))) ; If camera not shaking
    (if (Actor|ActorHasTag OtherActor "Wall")
      (Variables|Default|SetSpeed (* (Variables|Default|GetSpeed) 0.5))
      (ForceFeedback|SpawnForceFeedbackatLocation "/Game/Blueprints/CollVibrEffect.CollVibrEffect" "0, 0, 0" "0, 0, 0" false 1.0 0.0 0)
      (Variables|/Game/Blueprints/BP_PlayerCamera.BP_PlayerCamera_C|SetShaking (Variables|Default|GetCamera) true)
      (CallFunction|StopBoosting)
      (Class|AkGameplayStatics|StopActor _self)
      (Class|AkGameplayStatics|PostEvent "/Game/Audio/Player/Crash/Thuds.Thuds" _self)
      (else
        ;[1 1 1] Steam collision
        (bind _asbp_steam_system (Utilities|Casting|CastToBP_SteamSystem OtherActor))
        (Variables|/Game/Blueprints/BP_PlayerCamera.BP_PlayerCamera_C|SetBlurred _camera true)
        (Variables|/Game/Blueprints/BP_PlayerCamera.BP_PlayerCamera_C|SetTotalBlurTime _camera (Variables|/Game/SteamParticleFX/BP_SteamSystem.BP_SteamSystem_C|GetBlurDuration _asbp_steam_system))))))

(event EventBeginPlay
  ;[1 1 1] Enables input
  (Input|EnableInput (Game|GetPlayerController 0))
  (Variables|Default|SetDefaultSpeed (Variables|Default|GetMaxSpeed)))

(event EventTick
  (params (DeltaSeconds :type Float%20%28single-precision%29))
  (bind _self self)
  (bind _camera (Variables|Default|GetCamera))
  (bind _fuelmanagerref (Variables|Default|GetFuelManagerRef))
  (bind _radius (Variables|Default|GetRadius))
  (bind _player (Variables|Default|GetPlayer))
  (bind _yclamp (Variables|Default|GetYclamp))
  (bind _zclamp (Variables|Default|GetZclamp))
  (bind _camera_2 (Variables|Default|GetCamera))
  (bind _returnvalue (Transformation|GetRelativeTransform _player))
  (bind _fuel (Variables|/Game/Shield_demo/Fuel_Manager_Blueprint.Fuel_Manager_Blueprint_C|GetFuel _fuelmanagerref))
  ;[1 1 1] Makes the player go forwards
  (bind _output_get (Variables|Default|SetDelta%20Seconds DeltaSeconds))
  (if (not (Variables|Default|GetTurning))
    (Transformation|SetActorLocation (.newPos (Utilities|CalculateNewPos _output_get (Variables|Default|GetAcceleration) (Variables|Default|GetSpeed) (Transformation|GetWorldLocation (Variables|Default|GetOrigin)) (Math|Vector|RotateVector (Variables|Default|GetDirection) (Transformation|GetActorRotation)))) true false)
    (Variables|Default|SetSpeed (.newSpeed (Utilities|CalculateNewPos _output_get (Variables|Default|GetAcceleration) (Variables|Default|GetSpeed) (Transformation|GetWorldLocation (Variables|Default|GetOrigin)) (Math|Vector|RotateVector (Variables|Default|GetDirection) (Transformation|GetActorRotation)))))
    ;[1 1 1] Boost
    ;;[1 1 1] Decrement fuel if boosting
    (if (Variables|Default|GetBoosting)
      (Utilities|DecrementFloatby (Variables|/Game/Shield_demo/Fuel_Manager_Blueprint.Fuel_Manager_Blueprint_C|GetFuel _fuelmanagerref) (* (Variables|Default|GetDelta%20Seconds) (Variables|Default|GetFuelConsumption))
        (:OutExec
          ;;[1 1 1] If no fuel or fuel < desired fuel, set slowing
          (if (or (<= _fuel 0.0) (<= _fuel (Variables|Default|GetDesiredFuel)))
            (Variables|Default|SetSlowing true)
            (Variables|Default|SetBoosting false)
            (Class|AkGameplayStatics|StopActor _self)
            (Class|AkGameplayStatics|PostEvent "/Game/Audio/Player/Boost/Boost_End.Boost_End" _self)
            ;;[1 1 1] Slow down
            (Rendering|SetVisibility (Variables|Default|GetBoostParticle) false false)
            (if (Variables|Default|GetSlowing) :!label _label
              (CallFunction|SlowDown (Variables|Default|GetMaxSpeed) (Variables|Default|GetDefaultSpeed))))))
      (else
        (goto _label)))
    (if (Variables|Default|GetFreeMovement)
      ;[1 1 1] Sets the position
      (Transformation|SetRelativeLocation (Variables|Default|GetPlayer) (Math|Vector|MakeVector 0.0 (Math|Float|Clamp(Float) (+ (* (Variables|/Game/Blueprints/BP_PlayerCamera.BP_PlayerCamera_C|GetJoystick_X _camera) (Variables|Default|GetFreeMoveSpeed) (Variables|Default|GetDelta%20Seconds)) (.y (.location _returnvalue))) (* _yclamp -1.0) _yclamp) (Math|Float|Clamp(Float) (+ (.z (.location _returnvalue)) (* (Variables|/Game/Blueprints/BP_PlayerCamera.BP_PlayerCamera_C|GetJoystick_Y _camera) (Variables|Default|GetFreeMoveSpeed) (Variables|Default|GetDelta%20Seconds))) (* _zclamp -1.0) _zclamp)) false false)
      (else
        ;[1 1 1] Sets the position of the player based on the position of the joystick
        (Components|MoveComponentTo (Variables|Default|GetPlayer) (Math|Vector|MakeVector 0.0 (* (Variables|/Game/Blueprints/BP_PlayerCamera.BP_PlayerCamera_C|GetJoystick_X _camera_2) _radius) (* _radius (Variables|/Game/Blueprints/BP_PlayerCamera.BP_PlayerCamera_C|GetJoystick_Y _camera_2))) "0, 0, 0" false false 0.1 false)))))

(fn ConstructionScript)

(fn GetPlayerMiddle
  (return (Variables|Default|GetOrigin)))

(fn SlowDown
  (params (StartSpeed :type Float%20%28single-precision%29) (EndSpeed :type Float%20%28single-precision%29))
  ;[1 1 1] Slow down
  (Variables|Default|SetSlowing true)
  (Variables|Default|SetBoosting false)
  (bind _output_get (Variables|Default|SetMaxSpeed (Math|Float|Lerp StartSpeed EndSpeed (* (Variables|Default|GetDelta%20Seconds) (Variables|Default|GetDeccelSpeed)))))
  (if (Math|Float|NearlyEqual(Float) _output_get (Variables|Default|GetDefaultSpeed) 1e-06)
    (Variables|Default|SetSlowing false)
    (return)))

(fn SetSpeed
  (params (speed :type Float%20%28single-precision%29))
  (Variables|Default|SetSpeed (Math|Float|Clamp(Float) speed 0.0 (Variables|Default|GetMaxSpeed)))
  (return))

(fn StopBoosting
  (bind _self self)
  (if (Variables|Default|GetBoosting)
    (Variables|Default|SetSlowing true)
    (Variables|Default|SetBoosting false)
    (Rendering|SetVisibility (Variables|Default|GetBoostParticle) false false)
    (Class|AkGameplayStatics|StopActor _self)
    (Class|AkGameplayStatics|PostEvent "/Game/Audio/Player/Boost/Boost_End.Boost_End" _self)))