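; TurnManager actor that smoothly moves and rotates the referenced player onto a new axis while a turn is active.
; Each Tick while Turning, LerpAxis eases location toward DesiredPos on two axes, leaving the axis named by TurnEnum untouched.
; Rotation then lerps along the shortest path to DesiredRot, snapping and clearing Turning within tolerance.
; Both lerps use DeltaTime times MoveSpeed as alpha; completion checks rotation only.
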(event Collision|EventActorBeginOverlap
  (params (OtherActor :type Actor%20Object%20Reference)))

(event EventTick
  (params (DeltaSeconds :type Float%20%28single-precision%29))
  (bind _playerreference (Variables|Default|GetPlayerReference))
  (bind _desiredrot (Variables|Default|GetDesiredRot))
  (if (Variables|Default|GetTurning)
    ;[1 1 1] Lerp position to new axis
    (Variables|Default|SetDeltaTime DeltaSeconds)
    (Utilities|LerpAxis (Variables|Default|GetPlayerReference) (Variables|Default|GetDesiredPos) (Variables|Default|GetTurnEnum)
      (:OutExec
        ;[1 1 1] Lerp rotation
        (Transformation|SetActorRotation _playerreference (Math|Rotator|Lerp(Rotator) (Transformation|GetActorRotation _playerreference) (Variables|Default|GetDesiredRot) (* (Variables|Default|GetDeltaTime) (Variables|Default|GetMoveSpeed)) true))
        ;[1 1 1] Check if we are ready to stop rotating, if so, set rot to new rot and set Turning to false
        (if (Math|Rotator|Equal(Rotator) (Transformation|GetActorRotation (Variables|Default|GetPlayerReference)) _desiredrot 0.1)
          (Transformation|SetActorRotation (Variables|Default|GetPlayerReference) _desiredrot)
          (Variables|Default|SetTurning false))))))

(fn ConstructionScript)