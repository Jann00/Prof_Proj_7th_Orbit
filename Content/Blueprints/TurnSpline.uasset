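; Turn trigger actor that carries the player along a spline while its own camera films the turn.
; Box overlap stops boosting, flags the player as turning and blends the view to this actor.
; A Tick-started timeline eases the player toward spline positions with delta-scaled lerps, snapping at the end, as the camera tracks them.
; Leaving the box blends back to the player camera and resets player scale.
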(event OnComponentBeginOverlap(Box)
  (params (OverlappedComponent :type Primitive%20Component%20Object%20Reference) (OtherActor :type Actor%20Object%20Reference) (OtherComp :type Primitive%20Component%20Object%20Reference) (OtherBodyIndex :type Integer) (bFromSweep :type Boolean) (SweepResult :type Hit%20Result%20Structure%20%28by%20ref%29))
  (bind _asbp_player_movement (Utilities|Casting|CastToBP_PlayerMovement OtherActor))
  (if (Utilities|IsValid _asbp_player_movement)
    (bind _output_get (Variables|Default|SetPlayerRef _asbp_player_movement))
    (Default|StopBoosting _output_get)
    (Variables|Default|SetTurning true)
    (Variables|/Game/Blueprints/BP_PlayerMovement.BP_PlayerMovement_C|SetTurning _output_get true)
    (Components|Timeline|SetPlayRate (Variables|Default|GetTimeline_0) (Variables|Default|GetPlayRate))
    (bind _asplayer_controller (Utilities|Casting|CastToPlayerController (Pawn|GetController (Variables|/Game/Blueprints/BP_PlayerMovement.BP_PlayerMovement_C|GetCamera _output_get))))
    (if (Utilities|IsValid _asplayer_controller)
      (Game|Player|SetViewTargetwithBlend _asplayer_controller self (Variables|Default|GetCameraBlendTime) "VTBlend_Linear" 0.0 false))))

(event OnComponentEndOverlap(Box)
  (params (OverlappedComponent :type Primitive%20Component%20Object%20Reference) (OtherActor :type Actor%20Object%20Reference) (OtherComp :type Primitive%20Component%20Object%20Reference) (OtherBodyIndex :type Integer))
  (bind _asbp_player_movement (Utilities|Casting|CastToBP_PlayerMovement OtherActor))
  (if (Utilities|IsValid _asbp_player_movement)
    (bind _asplayer_controller (Utilities|Casting|CastToPlayerController (Pawn|GetController (Variables|/Game/Blueprints/BP_PlayerMovement.BP_PlayerMovement_C|GetCamera _asbp_player_movement))))
    (if (Utilities|IsValid _asplayer_controller)
      (Game|Player|SetViewTargetwithBlend _asplayer_controller (Variables|/Game/Blueprints/BP_PlayerMovement.BP_PlayerMovement_C|GetCamera _asbp_player_movement) (Variables|Default|GetCameraBlendTime) "VTBlend_Linear" 0.0 false)
      (Transformation|SetActorScale3D (Variables|Default|GetPlayerRef) "1.000000,1.000000,1.000000") ; Reset scale (in case we altered scale during turn)
    )))

(event EventBeginPlay
  (bind _returnvalue (Actor|GetActorOfClass "/Game/Blueprints/BP_PlayerMovement.BP_PlayerMovement_C"))
  (Variables|Default|SetPlayerRef _returnvalue))

(event Collision|EventActorBeginOverlap
  (params (OtherActor :type Actor%20Object%20Reference)))

(event EventTick
  (params (DeltaSeconds :type Float%20%28single-precision%29))
  (bind _playerref (Variables|Default|GetPlayerRef))
  (Variables|Default|SetDelta%20Seconds DeltaSeconds)
  (if (Variables|Default|GetTurning)
    (bind _alpha (Timeline|Timeline_0 Play)
      (:Update
        (bind _output_get (Variables|Default|SetAlpha _alpha))
        (bind _done (CallFunction|LerpAlongSpline (Variables|Default|GetPlayerRef) (Variables|Default|GetPlayerSpline) _output_get))
        (if _done
          (Variables|Default|SetTurning false)
          (Variables|/Game/Blueprints/BP_PlayerMovement.BP_PlayerMovement_C|SetTurning _playerref false))
        (CallFunction|RotateCamtoTarget (Variables|Default|GetBP_TurnCameraActor) (Variables|/Game/Blueprints/BP_PlayerMovement.BP_PlayerMovement_C|GetPlayer _playerref))))))

(fn ConstructionScript)

(fn LerpAlongSpline
  (params (Actor :type Actor%20Object%20Reference) (Spline :type Spline%20Component%20Object%20Reference) (Alpha :type Float%20%28single-precision%29))
  (Transformation|SetActorTransform Actor (Math|Transform|Lerp(Transform) (Transformation|GetActorTransform Actor) (Spline|GetTransformatDistanceAlongSpline Spline (Math|Float|Lerp 0.0 (Spline|GetSplineLength Spline) Alpha) "World" false) (Math|Float|NormalizetoRange (* (Variables|Default|GetDelta%20Seconds) 1e+01) 0.0 1.0)))
  (if (>= Alpha 1.0)
    (Variables|Default|SetDone true)
    (Transformation|SetActorTransform Actor (Spline|GetTransformatSplinePoint Spline (Spline|GetNumberOfSplinePoints Spline) "World" false))
    (else
      (Variables|Default|SetDone false)))
  (return (Variables|Default|GetDone)))

(fn RotateCamtoTarget
  (params (Camera :type BP%20Turn%20Camera%20Actor%20Object%20Reference) (Target :type Static%20Mesh%20Component%20Object%20Reference))
  (Transformation|SetWorldRotation Camera (Math|Rotator|Lerp(Rotator) (Transformation|GetWorldRotation Camera) (Math|Rotator|FindLookatRotation (Transformation|GetWorldLocation Camera) (Transformation|GetWorldLocation Target)) (Variables|Default|GetCameraTrackingAlpha) true) false false))