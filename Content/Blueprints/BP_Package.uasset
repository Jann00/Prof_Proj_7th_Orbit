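; BP_Package is a package that attaches to the player at BeginPlay and tumbles away, then explodes, once its Falling flag is set.
; BeginPlay finds BP_PlayerMovement, attaches to its Player component and picks a random fall direction.
; While Falling, Tick calls FallOff with speed and spin multipliers re-rolled every frame.
; FallOff moves and spins the mesh, counts down DeathTimer, then spawns an explosion with Wwise audio and destroys the actor.
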(event EventBeginPlay
  (bind _returnvalue (Actor|GetActorOfClass "/Game/Blueprints/BP_PlayerMovement.BP_PlayerMovement_C"))
  (Variables|Default|SetPlayer _returnvalue)
  (Transformation|AttachComponentToComponent (Variables|/Game/Blueprints/BP_PlayerMovement.BP_PlayerMovement_C|GetPlayer _returnvalue) "None" "KeepWorld" "KeepWorld" "KeepWorld" false)
  (Variables|Default|SetFallSpeed (* (Math|Random|RandomUnitVector) 5e+03)))

(event Collision|EventActorBeginOverlap
  (params (OtherActor :type Actor%20Object%20Reference)))

(event EventTick
  (params (DeltaSeconds :type Float%20%28single-precision%29))
  (bind _returnvalue (Math|Random|RandomFloatinRange 1.0 3.0))
  (if (Variables|Default|GetFalling)
    (CallFunction|FallOff DeltaSeconds _returnvalue _returnvalue)))

(fn ConstructionScript)

(fn FallOff
  (params (DeltaTime :type Float%20%28single-precision%29) (FallSpeedMult :type Float%20%28single-precision%29) (SpinSpeedMult :type Float%20%28single-precision%29))
  (bind _packagemesh (Variables|Default|GetPackageMesh))
  (bind _fallspeed (Variables|Default|GetFallSpeed))
  (bind _returnvalue (* _fallspeed FallSpeedMult))
  (bind _returnvalue_2 (Transformation|GetWorldLocation _packagemesh))
  (Transformation|AddRelativeLocation (Variables|Default|GetPackageMesh) (* (Math|Vector|MakeVector (.x _returnvalue) (.y _returnvalue) (.z _returnvalue)) DeltaTime) false false)
  (Transformation|AddWorldRotation (Variables|Default|GetPackageMesh) (* "250.000000,200.000000,300.000000" (* SpinSpeedMult DeltaTime)) false false)
  (bind _output_get (Variables|Default|SetDeathTimer (- (Variables|Default|GetDeathTimer) DeltaTime)))
  (if (<= _output_get 0.0)
    (Effects|SpawnEmitteratLocation "/Game/StarterContent/Particles/P_Explosion.P_Explosion" _returnvalue_2 "0, 0, 0" "2.500000,2.500000,2.500000")
    (Class|AkGameplayStatics|PostEventatLocation "/Game/Audio/Enemy/Death_Explosions.Death_Explosions" _returnvalue_2 "0, 0, 0")
    (Actor|DestroyActor)))