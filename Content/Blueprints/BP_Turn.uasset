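; BP_Turn is a trigger that steers an overlapping BP_MovementCircle toward the axis direction set by its Turn enum.
; BeginPlay derives a target point on the Cube's bounds and a matching rotation from that enum.
; After overlap, Tick lerps the circle's two off-axis coordinates and its rotation, leaving the travel axis untouched.
; It destroys itself once rotation matches, but reaching the target point first halts both lerps.
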(event OnComponentBeginOverlap(Collide)
  (params (OverlappedComponent :type Primitive%20Component%20Object%20Reference) (OtherActor :type Actor%20Object%20Reference) (OtherComp :type Primitive%20Component%20Object%20Reference) (OtherBodyIndex :type Integer) (bFromSweep :type Boolean) (SweepResult :type Hit%20Result%20Structure%20%28by%20ref%29))
  (bind _asbp_movement_circle (Utilities|Casting|CastToBP_MovementCircle OtherActor))
  (Variables|Default|SetTranslating true)
  (Variables|Default|SetTurning true))

(event EventTick
  (params (DeltaSeconds :type Float%20%28single-precision%29))
  (bind _desiredpos (Variables|Default|GetDesiredPos))
  (bind _desiredrot (Variables|Default|GetDesiredRot))
  (if (not (Variables|Default|GetDone))
    (bind _output_get (Variables|Default|SetDeltaTime DeltaSeconds))
    (if (Variables|Default|GetTranslating)
      (Utilities|LerpAxis (stale OnComponentBeginOverlap(Collide) _asbp_movement_circle) _desiredpos (Variables|Default|GetTurn)
        (:OutExec
          (if (Utilities|IsinRange _desiredpos (Transformation|GetActorLocation (stale OnComponentBeginOverlap(Collide) _asbp_movement_circle)) 1.0)
            (Variables|Default|SetTurning false)
            (Variables|Default|SetTranslating false)
            (else
              (if (Variables|Default|GetTurning) :!label _label
                (Transformation|SetActorRotation (stale OnComponentBeginOverlap(Collide) _asbp_movement_circle) (Math|Rotator|Lerp(Rotator) (Transformation|GetActorRotation (stale OnComponentBeginOverlap(Collide) _asbp_movement_circle)) (Variables|Default|GetDesiredRot) (* _output_get (Variables|Default|GetMoveSpeed)) true))
                (if (Math|Rotator|Equal(Rotator) (Transformation|GetActorRotation (stale OnComponentBeginOverlap(Collide) _asbp_movement_circle)) _desiredrot 0.1)
                  (Transformation|SetActorRotation (stale OnComponentBeginOverlap(Collide) _asbp_movement_circle) _desiredrot)
                  (Variables|Default|SetDone true)
                  (Actor|DestroyActor)))))))
      (else
        (goto _label)))))

(event EventBeginPlay
  (bind _returnvalue (Transformation|GetActorLocation))
  (bind _cube (Variables|Default|GetCube))
  (bind _boxextent (Collision|GetComponentBounds _cube))
  ;[1 1 1] Set Desired Pos from Enum
  (switch Utilities|FlowControl|Switch|SwitchonTurnEnum (Variables|Default|GetTurn)
    (:NewEnumerator0
      ;;[1 1 1 1 12] +Y/-Y
      (Variables|Default|SetDesiredPos (Math|Vector|MakeVector (.x _returnvalue) (+ (.y _returnvalue) (.y _boxextent)) (.z _returnvalue)))
      (Variables|Default|SetDesiredRot "0,90.000000, 0"))
    (:NewEnumerator1
      (Variables|Default|SetDesiredPos (Math|Vector|MakeVector (.x _returnvalue) (- (.y _returnvalue) (.y _boxextent)) (.z _returnvalue)))
      (Variables|Default|SetDesiredRot "0,-90.000000, 0"))
    (:NewEnumerator2
      ;;[1 1 1 1 12] +Z/-Z
      (Variables|Default|SetDesiredPos (Math|Vector|MakeVector (.x _returnvalue) (.y _returnvalue) (+ (.z _returnvalue) (.z _boxextent))))
      (Variables|Default|SetDesiredRot "90.000000, 0,0.000000"))
    (:NewEnumerator3
      (Variables|Default|SetDesiredPos (Math|Vector|MakeVector (.x _returnvalue) (.y _returnvalue) (- (.z _returnvalue) (.z _boxextent))))
      (Variables|Default|SetDesiredRot "-90.000000, 0,0.000000"))
    (:NewEnumerator4
      ;;[1 1 1 1 12] +X/-X
      (Variables|Default|SetDesiredPos (Math|Vector|MakeVector (+ (.x _returnvalue) (.x _boxextent)) (.y _returnvalue) (.z _returnvalue)))
      (Variables|Default|SetDesiredRot "0, 0, 0"))
    (:NewEnumerator5
      (Variables|Default|SetDesiredPos (Math|Vector|MakeVector (- (.x _returnvalue) (.x _boxextent)) (.y _returnvalue) (.z _returnvalue)))
      (Variables|Default|SetDesiredRot "0,180.000000, 0"))))

(fn ConstructionScript)