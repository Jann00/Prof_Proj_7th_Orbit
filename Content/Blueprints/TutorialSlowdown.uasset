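; Tutorial trigger actor that slows game time to a stop when the player enters its box, until a required input is given.
; The first BP_PlayerMovement overlap runs a one-time timeline that lerps global time dilation to zero.
; Flags select which inputs (laser, boost/shield, or left stick past half deflection, polled on Tick) play a second timeline restoring normal speed.
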(event OnComponentBeginOverlap(Box)
  (params (OverlappedComponent :type Primitive%20Component%20Object%20Reference) (OtherActor :type Actor%20Object%20Reference) (OtherComp :type Primitive%20Component%20Object%20Reference) (OtherBodyIndex :type Integer) (bFromSweep :type Boolean) (SweepResult :type Hit%20Result%20Structure%20%28by%20ref%29))
  (if (not (Variables|Default|GetSlowDown))
    (Utilities|Casting|CastToBP_PlayerMovement OtherActor)
    (Variables|Default|SetSlowDown true)
    (bind _time (Timeline|Timeline_0 PlayFromStart)
      (:Update
        (Utilities|Time|SetGlobalTimeDilation (Math|Float|Lerp 1.0 0.0 _time))
        (Variables|Default|SetTimeResumed false)))))

(event EventBeginPlay
  (Input|EnableInput (Game|GetPlayerController 0)))

(event Collision|EventActorBeginOverlap
  (params (OtherActor :type Actor%20Object%20Reference)))

(event EventTick
  (params (DeltaSeconds :type Float%20%28single-precision%29))
  (bind _returnvalue (Input|AxisValues|GetLeft_Joystick_X))
  (bind _returnvalue_2 (Input|AxisValues|GetLeft_Joystick_Y))
  (Math|Float|CompareFloat _returnvalue 0.5
    (:>
      _)
    (:==
      _)
    (:<
      (Math|Float|CompareFloat _returnvalue -0.5
        (:>
          (Math|Float|CompareFloat _returnvalue_2 0.5
            (:>
              _)
            (:==
              _)
            (:<
              (Math|Float|CompareFloat _returnvalue_2 -0.5
                (:==
                  _)
                (:<
                  _)))))
        (:==
          _)
        (:<
          _))))
  (if (Variables|Default|GetMoveToEnd)
    (if (not (Variables|Default|GetTimeResumed))
      (Variables|Default|SetTimeResumed true)
      (bind _time (Timeline|Timeline_1 PlayFromStart)
        (:Update
          (Utilities|Time|SetGlobalTimeDilation (Math|Float|Lerp 0.0 1.0 _time)))))))

(event Input|ActionEvents|InputActionBoost/Shield
  (params (Key :type Key%20Structure :default "None"))
  (:Pressed
    (if (Variables|Default|GetBoostToEnd)
      (if (not (Variables|Default|GetTimeResumed))
        (Variables|Default|SetTimeResumed true)
        (bind _time (Timeline|Timeline_1 PlayFromStart)
          (:Update
            (Utilities|Time|SetGlobalTimeDilation (Math|Float|Lerp 0.0 1.0 _time))))))))

(event Input|ActionEvents|InputActionShootLaser
  (params (Key :type Key%20Structure :default "None"))
  (:Pressed
    (if (Variables|Default|GetLaserToEnd)
      (if (not (Variables|Default|GetTimeResumed))
        (Variables|Default|SetTimeResumed true)
        (bind _time (Timeline|Timeline_1 PlayFromStart)
          (:Update
            (Utilities|Time|SetGlobalTimeDilation (Math|Float|Lerp 0.0 1.0 _time))))))))

(fn ConstructionScript)