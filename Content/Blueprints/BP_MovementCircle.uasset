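; Player movement rig that drives the actor forward with swept moves while the joystick shifts its Cube sideways and vertically.
; Tick feeds CalculateNewPos for speed and position, then either moves the Cube freely within Y/Z clamps or eases it to a radius-scaled stick offset.
; Boosting drains the tagged player shield's fuel; running out lerps max speed down.
; Overlapping a Wall-tagged actor cuts speed and plays force feedback.
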(event OnComponentBeginOverlap(Cube)
  (params (OverlappedComponent :type Primitive%20Component%20Object%20Reference) (OtherActor :type Actor%20Object%20Reference) (OtherComp :type Primitive%20Component%20Object%20Reference) (OtherBodyIndex :type Integer) (bFromSweep :type Boolean) (SweepResult :type Hit%20Result%20Structure%20%28by%20ref%29))
  ;[1 1 1] Wall collision
  (if (Actor|ActorHasTag OtherActor "Wall")
    (Variables|Default|SetSpeed (* (Variables|Default|GetSpeed) 0.25))
    (ForceFeedback|SpawnForceFeedbackatLocation "/Game/Blueprints/CollVibrEffect.CollVibrEffect" "0, 0, 0" "0, 0, 0" false 1.0 0.0 0)))

(event EventBeginPlay
  ;[1 1 1] Enables input
  (Input|EnableInput (Game|GetPlayerController 0))
  ;[1 1 1] Get shield reference
  (bind _outactors (Actor|GetAllActorswithTag "PlayerShield"))
  (bind _asplayer_shield (Utilities|Casting|CastToplayer_shield (Utilities|Array|Get(acopy) _outactors)))
  (Variables|Default|SetShieldRef _asplayer_shield))

(event EventTick
  (params (DeltaSeconds :type Float%20%28single-precision%29))
  (bind _camera (Variables|Default|GetCamera))
  (bind _radius (Variables|Default|GetRadius))
  (bind _shieldref (Variables|Default|GetShieldRef))
  (bind _cube (Variables|Default|GetCube))
  (bind _yclamp (Variables|Default|GetYclamp))
  (bind _zclamp (Variables|Default|GetZclamp))
  (bind _camera_2 (Variables|Default|GetCamera))
  (bind _returnvalue (Transformation|GetRelativeTransform _cube))
  ;[1 1 1] Makes the player go forwards
  (bind _output_get (Variables|Default|SetDelta%20Seconds DeltaSeconds))
  ;[1 1 1] Decrement fuel if boosting
  (if (Variables|Default|GetBoosting)
    (Utilities|DecrementFloatby (Variables|/Game/Shield_demo/player_shield.player_shield_C|GetFuel _shieldref) (* (Variables|Default|GetDelta%20Seconds) 1e+01)
      (:OutExec
        ;[1 1 1] Boost
        ;;[1 1 1] If no fuel, set slowing
        (Variables|Default|SetSlowing (<= (Variables|/Game/Shield_demo/player_shield.player_shield_C|GetFuel _shieldref) 0.0)))))
  ;;[1 1 1] Slow down
  (if (Variables|Default|GetSlowing)
    (bind _output_get_2 (Variables|Default|SetMaxSpeed (Math|Float|Lerp (Variables|Default|GetMaxSpeed) 5e+01 (* (Variables|Default|GetDelta%20Seconds) (Variables|Default|GetDeccelSpeed)))))
    (if (Math|Float|NearlyEqual(Float) _output_get_2 5e+01 1e-06)
      (Variables|Default|SetSlowing false)))
  (Transformation|SetActorLocation (.newPos (Utilities|CalculateNewPos _output_get (Variables|Default|GetAcceleration) (Variables|Default|GetSpeed) (Transformation|GetWorldLocation (Variables|Default|GetCube1)) (Math|Vector|RotateVector (Variables|Default|GetDirection) (Transformation|GetActorRotation)))) true false)
  (Variables|Default|SetSpeed (.newSpeed (Utilities|CalculateNewPos _output_get (Variables|Default|GetAcceleration) (Variables|Default|GetSpeed) (Transformation|GetWorldLocation (Variables|Default|GetCube1)) (Math|Vector|RotateVector (Variables|Default|GetDirection) (Transformation|GetActorRotation)))))
  (if (Variables|Default|GetFreeMovement)
    ;[1 1 1] Sets the position
    (Transformation|SetRelativeLocation (Variables|Default|GetCube) (Math|Vector|MakeVector 0.0 (Math|Float|Clamp(Float) (+ (* (Variables|/Game/Blueprints/BP_PlayerCamera.BP_PlayerCamera_C|GetJoystick_X _camera) (Variables|Default|GetFreeMoveSpeed) (Variables|Default|GetDelta%20Seconds)) (.y (.location _returnvalue))) (* _yclamp -1.0) _yclamp) (Math|Float|Clamp(Float) (+ (.z (.location _returnvalue)) (* (Variables|/Game/Blueprints/BP_PlayerCamera.BP_PlayerCamera_C|GetJoystick_Y _camera) (Variables|Default|GetFreeMoveSpeed) (Variables|Default|GetDelta%20Seconds))) (* _zclamp -1.0) _zclamp)) false false)
    (else
      ;[1 1 1] Sets the position of the player based on the position of the joystick
      (Components|MoveComponentTo (Variables|Default|GetCube) (Math|Vector|MakeVector 0.0 (* (Variables|/Game/Blueprints/BP_PlayerCamera.BP_PlayerCamera_C|GetJoystick_X _camera_2) _radius) (* _radius (Variables|/Game/Blueprints/BP_PlayerCamera.BP_PlayerCamera_C|GetJoystick_Y _camera_2))) "0, 0, 0" false false 0.1 false))))

(fn ConstructionScript)

(fn GetPlayerMiddle
  (return (Variables|Default|GetCube1)))