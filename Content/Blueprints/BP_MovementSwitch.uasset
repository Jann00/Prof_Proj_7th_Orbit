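; BP_MovementSwitch is a trigger that switches the player between free-movement fighting sections and regular movement.
; On player overlap it switches the Turbo_Song Wwise music state, refills fuel and sets the FreeMovement flag from EnableFreeMovement.
; Entering activates the enemy zone, assigns the fighting path and stops boosting.
; Leaving deactivates the zone, realigns the player to PostSwitchDirection and resets spline distance.
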(event OnComponentBeginOverlap(Collide)
  (params (OverlappedComponent :type Primitive%20Component%20Object%20Reference) (OtherActor :type Actor%20Object%20Reference) (OtherComp :type Primitive%20Component%20Object%20Reference) (OtherBodyIndex :type Integer) (bFromSweep :type Boolean) (SweepResult :type Hit%20Result%20Structure%20%28by%20ref%29))
  (bind _enemyzoneref (Variables|Default|GetEnemyZoneRef))
  (bind _enablefreemovement (Variables|Default|GetEnableFreeMovement))
  (bind _postswitchdirection (Variables|Default|GetPostSwitchDirection))
  (bind _returnvalue (Transformation|GetWorldRotation _postswitchdirection))
  (bind _asbp_player_movement (Utilities|Casting|CastToBP_PlayerMovement OtherActor))
  (bind _returnvalue_2 (Actor|GetActorOfClass "/Game/Shield_demo/Fuel_Manager_Blueprint.Fuel_Manager_Blueprint_C"))
  (Class|AkComponent|SetSwitch (Variables|/Game/Shield_demo/Fuel_Manager_Blueprint.Fuel_Manager_Blueprint_C|GetMusic _returnvalue_2) 0 "Turbo_Song" (Variables|Default|GetSongToSwitchTo))
  (bind _output_get (Variables|Default|SetPlayerRef _asbp_player_movement))
  (Variables|/Game/Blueprints/BP_PlayerMovement.BP_PlayerMovement_C|SetFreeMovement _asbp_player_movement _enablefreemovement)
  (Variables|/Game/Shield_demo/Fuel_Manager_Blueprint.Fuel_Manager_Blueprint_C|SetFuel (Variables|/Game/Blueprints/BP_PlayerMovement.BP_PlayerMovement_C|GetFuelManagerRef (Variables|Default|GetPlayerRef)) 1e+02)
  (if _enablefreemovement
    ;[1 1 1] Setup zone (attach to player, disable boosting)
    (Default|ActivateZone _enemyzoneref _output_get)
    (Variables|/Game/Blueprints/BP_PlayerMovement.BP_PlayerMovement_C|SetFightingSectionPath (Variables|Default|GetPlayerRef) (Variables|Default|GetMovePath))
    (if (Variables|/Game/Blueprints/BP_PlayerMovement.BP_PlayerMovement_C|GetBoosting (Variables|Default|GetPlayerRef))
      (Default|StopBoosting (Variables|Default|GetPlayerRef)))
    (else
      ;[1 1 1] Reached end of this zone, deassgin and clear up enemies
      (Default|DeactivateZone _enemyzoneref)
      (Variables|/Game/Blueprints/BP_PlayerMovement.BP_PlayerMovement_C|SetDirection (Variables|Default|GetPlayerRef) (Math|Rotator|GetRotationXVector _returnvalue))
      (Transformation|SetWorldRotation (Variables|/Script/Engine.Actor|GetRootComponent (Variables|Default|GetPlayerRef)) _returnvalue false false)
      (Variables|/Game/Blueprints/BP_PlayerMovement.BP_PlayerMovement_C|SetsplineDistanceTravelled (Variables|Default|GetPlayerRef) 0.0))))

(event EventBeginPlay)

(event Collision|EventActorBeginOverlap
  (params (OtherActor :type Actor%20Object%20Reference)))

(event EventTick
  (params (DeltaSeconds :type Float%20%28single-precision%29)))

(fn ConstructionScript)