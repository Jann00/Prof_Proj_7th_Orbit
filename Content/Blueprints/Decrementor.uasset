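; Decrementor is a Blueprint timer that, despite its name, counts elapsed time upward in Minutes and Seconds.
; Tick runs through a one-second Delay, so the counter advances roughly once per second.
; Seconds increments until it reaches 59, then resets to zero and adds a minute if Minutes is non-negative.
; The Decrement function is an empty stub.
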(event EventBeginPlay)

(event Collision|EventActorBeginOverlap
  (params (OtherActor :type Actor%20Object%20Reference)))

(event EventTick
  (params (DeltaSeconds :type Float%20%28single-precision%29))
  (Utilities|FlowControl|Delay 1.0)
  (if (== (Variables|Default|GetSeconds) 59)
    (if (>= (Variables|Default|GetMinutes) 0)
      (Variables|Default|SetSeconds 0)
      (Variables|Default|SetMinutes (+ (Variables|Default|GetMinutes) 1)))
    (else
      (Variables|Default|SetSeconds (+ (Variables|Default|GetSeconds) 1)))))

(fn ConstructionScript)

(fn Decrement)