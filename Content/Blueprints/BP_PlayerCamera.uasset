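; Player camera actor that follows PlayerMovement each tick, widens FOV with speed and also handles Boost input.
; Camera offset tracks the movement Cube in free movement, or eases toward left-stick input scaled by Radius when locked.
; Flag-driven, timed effects add random rotation shake scaled by speed and remaining time, and blur by lerping post-process focal distance.
; Boost spends fuel on press, jumps speed and sets PlayerMovement's boosting state, switching to slowing on release.
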(event EventBeginPlay
  ;[1 1 1] Enables input
  (Input|EnableInput (Game|GetPlayerController 0))
  ;[1 1 1] Set timers
  (Variables|Default|SetShakeTimer (Variables|Default|GetTotalShakeTime)))

(event Collision|EventActorBeginOverlap
  (params (OtherActor :type Actor%20Object%20Reference)))

(event EventTick
  (params (DeltaSeconds :type Float%20%28single-precision%29))
  (bind _playermovement (Variables|Default|GetPlayerMovement))
  (bind _camera (Variables|Default|GetCamera))
  (bind _playermovement_2 (Variables|Default|GetPlayerMovement))
  (bind _playermovement_3 (Variables|Default|GetPlayerMovement))
  (bind _playermovement_4 (Variables|Default|GetPlayerMovement))
  (bind _returnvalue (Transformation|GetRelativeTransform _camera))
  (bind _returnvalue_2 (Transformation|GetActorTransform _playermovement_4))
  (bind _cube (Variables|/Game/Blueprints/BP_MovementCircle.BP_MovementCircle_C|GetCube _playermovement))
  (bind _radius (Variables|/Game/Blueprints/BP_MovementCircle.BP_MovementCircle_C|GetRadius _playermovement_3))
  (bind _returnvalue_3 (Transformation|GetRelativeTransform _cube))
  (Variables|Default|SetDelta%20Seconds DeltaSeconds)
  ;[1 1 1] Speed based FOV
  (Variables|/Script/Engine.CameraComponent|SetFieldOfView (Variables|Default|GetCamera) (Math|Float|Lerp (Variables|Default|GetDefaultFov) (Variables|Default|GetMaxFov) (/ (Variables|/Game/Blueprints/BP_MovementCircle.BP_MovementCircle_C|GetSpeed _playermovement_2) (Variables|/Game/Blueprints/BP_MovementCircle.BP_MovementCircle_C|GetBoostSpeed _playermovement_2))))
  (Variables|Default|SetJoystick_X (Input|AxisValues|GetLeft_Joystick_X))
  (Variables|Default|SetJoystick_Y (Input|AxisValues|GetLeft_Joystick_Y))
  (Transformation|SetActorLocationAndRotation (.location _returnvalue_2) (.rotation _returnvalue_2))
  ;[1 1 1] Shake camera
  (if (Variables|Default|GetShaking)
    (CallFunction|Shake))
  ;[1 1 1] Blur
  (if (Variables|Default|GetBlurred)
    (CallFunction|Blur))
  (if (Variables|/Game/Blueprints/BP_MovementCircle.BP_MovementCircle_C|GetFreeMovement (Variables|Default|GetPlayerMovement))
    ;[1 1 1] Free movement camera
    (Transformation|SetRelativeLocation (Variables|Default|GetCamera) (Math|Vector|MakeVector -1e+03 (/ (.y (.location _returnvalue_3)) 3.0) (+ (/ (.z (.location _returnvalue_3)) 2.0) 2e+02)) false false)
    (else
      ;[1 1 1] Locked movement camera
      (Transformation|SetRelativeLocation _camera (Math|Vector|MakeVector (Variables|Default|GetCameraOffset) (Math|Interpolation|Ease "Linear" (* (Variables|Default|GetDelta%20Seconds) 3.0) (.y (.location _returnvalue)) (/ (* (Input|AxisValues|GetLeft_Joystick_X) _radius) 2.0)) (Math|Interpolation|Ease "Linear" (* (Variables|Default|GetDelta%20Seconds) 3.0) (.z (.location _returnvalue)) (+ (/ (* _radius (Input|AxisValues|GetLeft_Joystick_Y)) 2.0) 2e+02))) false false))))

(event Input|ActionEvents|InputActionBoost
  (params (Key :type Key%20Structure :default "None"))
  (bind _playermovement (Variables|Default|GetPlayerMovement))
  (bind _playermovement_2 (Variables|Default|GetPlayerMovement))
  (bind _playermovement_3 (Variables|Default|GetPlayerMovement))
  (bind _fuelmanagerref (Variables|/Game/Blueprints/BP_MovementCircle.BP_MovementCircle_C|GetFuelManagerRef _playermovement_3))
  ;[1 1 1] Boost
  (:Pressed
    ;;[1 1 1] If fuel>min, start boosting, multiply speed initially by 1.5
    (if (> (Variables|/Game/Shield_demo/Fuel_Manager_Blueprint.Fuel_Manager_Blueprint_C|GetFuel (Variables|/Game/Blueprints/BP_MovementCircle.BP_MovementCircle_C|GetFuelManagerRef (Variables|Default|GetPlayerMovement))) (Variables|Default|GetFuelPressCost))
      (Variables|/Game/Blueprints/BP_MovementCircle.BP_MovementCircle_C|SetMaxSpeed _playermovement_2 (Variables|/Game/Blueprints/BP_MovementCircle.BP_MovementCircle_C|GetBoostSpeed _playermovement_2))
      (Default|SetSpeed _playermovement_3 (* (Variables|/Game/Blueprints/BP_MovementCircle.BP_MovementCircle_C|GetSpeed _playermovement_3) 1.5))
      ;;[1 1 1] Decrement fuel
      (Variables|/Game/Blueprints/BP_MovementCircle.BP_MovementCircle_C|SetSlowing _playermovement_3 false)
      (Variables|/Game/Shield_demo/Fuel_Manager_Blueprint.Fuel_Manager_Blueprint_C|SetFuel _fuelmanagerref (- (Variables|/Game/Shield_demo/Fuel_Manager_Blueprint.Fuel_Manager_Blueprint_C|GetFuel _fuelmanagerref) (Variables|Default|GetFuelPressCost)))
      (Variables|/Game/Blueprints/BP_MovementCircle.BP_MovementCircle_C|SetBoosting _playermovement_3 true)))
  (:Released
    (Variables|/Game/Blueprints/BP_MovementCircle.BP_MovementCircle_C|SetBoosting _playermovement false)
    (Variables|/Game/Blueprints/BP_MovementCircle.BP_MovementCircle_C|SetSlowing _playermovement true)))

(fn ConstructionScript)

(fn SetRandomRotation
  (params (Amplitude :type Float%20%28single-precision%29))
  (bind _returnvalue (Math|Random|RandomUnitVector))
  (bind _returnvalue_2 (* _returnvalue Amplitude))
  (Transformation|SetActorRotation (Math|Rotator|MakeRotator (.x _returnvalue_2) (.y _returnvalue_2) (.z _returnvalue_2)))
  (return))

(fn StopShake
  (Variables|Default|SetShakeTimer (Variables|Default|GetTotalShakeTime))
  (Variables|Default|SetShaking false)
  (Transformation|SetActorRotation "0, 0, 0"))

(fn Shake
  ;[1 1 1] Shake camera
  (if (>= (Variables|Default|GetShakeTimer) 0.0)
    (bind _output_get (Variables|Default|SetShakeTimer (- (Variables|Default|GetShakeTimer) (Variables|Default|GetDelta%20Seconds))))
    (CallFunction|SetRandomRotation (* _output_get (Variables|Default|GetShakeAmp) (Variables|/Game/Blueprints/BP_MovementCircle.BP_MovementCircle_C|GetSpeed (Variables|Default|GetPlayerMovement))))
    (else
      (CallFunction|StopShake))))

(fn Blur
  (if (<= (Variables|Default|GetBlurTimer) (Variables|Default|GetTotalBlurTime))
    (Variables|Default|SetBlurTimer (+ (Variables|Default|GetBlurTimer) (Variables|Default|GetDelta%20Seconds)))
    (bind _output_get (LocalVariables|SetCurrentFocalDistance (Math|Float|Lerp (LocalVariables|GetCurrentFocalDistance) 2e+01 (Utilities|GetNormalizedTimer))))
    (Utilities|Struct|SetmembersinPostProcessSettings (Variables|/Script/Engine.PostProcessVolume|GetSettings (Variables|Default|GetPostProcessRef)) _output_get)
    (else
      (Variables|Default|SetBlurTimer 0.0)
      (Variables|Default|SetBlurred false)
      (Utilities|Struct|SetmembersinPostProcessSettings (Variables|/Script/Engine.PostProcessVolume|GetSettings (Variables|Default|GetPostProcessRef)) 0.0))))