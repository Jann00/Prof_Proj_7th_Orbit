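; BP_house_l10_01 is an assembled house actor that randomizes its window layout on BeginPlay.
; It loops through SharedRoot's child static mesh components and picks wall pieces by display name.
; Pieces named "wall_window" become blank walls, while "wall_blank" pieces randomly receive window meshes based on WindowSpawnChance.
; Each spawned window then gets a lit or unlit emissive material based on LitWindowChance.
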(event EventBeginPlay
  (for _array_element (Components|GetChildrenComponents (Variables|Default|GetSharedRoot) true)
    (bind _asstatic_mesh_component (Utilities|Casting|CastToStaticMeshComponent _array_element))
    (if (Utilities|String|Contains (Utilities|GetDisplayName _asstatic_mesh_component) "wall_window")
      (Components|StaticMesh|SetStaticMesh _asstatic_mesh_component "/Game/meshes/enviroment_assets/wall_blank.wall_blank"))
    (if (Utilities|String|Contains (Utilities|GetDisplayName _asstatic_mesh_component) "wall_blank")
      (if (<= (Math|Random|RandomFloat) (Variables|Default|GetwindowSpawnChance))
        (Components|StaticMesh|SetStaticMesh _asstatic_mesh_component "/Game/meshes/enviroment_assets/wall_window.wall_window")
        (if (<= (Math|Random|RandomFloat) (Variables|Default|GetlitWindowChance))
          (Rendering|Material|SetMaterial _asstatic_mesh_component 2 "/Game/Materials/MI_window_emissive.MI_window_emissive")
          (else
            (Rendering|Material|SetMaterial _asstatic_mesh_component 2 "/Game/Materials/MI_window_emissive_off.MI_window_emissive_off")))))))

(event Collision|EventActorBeginOverlap
  (params (OtherActor :type Actor%20Object%20Reference)))

(event EventTick
  (params (DeltaSeconds :type Float%20%28single-precision%29)))

(fn ConstructionScript)