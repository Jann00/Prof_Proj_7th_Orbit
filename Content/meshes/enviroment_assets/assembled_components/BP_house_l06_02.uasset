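; BP_house_l06_02 is an assembled house Blueprint that randomises its windows on BeginPlay.
; SpawnRandomWindows scans child static mesh components by name, resetting "wall_window" pieces to blank walls and randomly swapping "wall_blank" pieces to window meshes.
; New windows get a lit or unlit material by chance, with lit ones tinted through the Emissive_colour parameter in the main colour or occasionally one of two alternates.
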(event EventBeginPlay
  (CallFunction|SpawnRandomWindows (Variables|Default|GetwindowSpawnChance) (Variables|Default|GetlitWindowChance) (Variables|Default|GetUniqueWindowChance) (Variables|Default|GetMainColour) (Variables|Default|GetAltColour1) (Variables|Default|GetAltColour2) (Variables|Default|GetDefaultSceneRoot)))

(fn ConstructionScript)

(fn SpawnRandomWindows
  (params (windowSpawnChance_ :type Float%20%28single-precision%29) (litWindowChance_ :type Float%20%28single-precision%29) (uniqueWindowChance :type Float%20%28single-precision%29) (MainColour_ :type Color%20Structure) (AltColour1 :type Color%20Structure) (AltColour2 :type Color%20Structure) (Root :type Scene%20Component%20Object%20Reference))
  (bind _returnvalue (Math|Conversions|ToLinearColor(Color) MainColour_))
  (bind _returnvalue_2 (Math|Conversions|ToLinearColor(Color) AltColour2))
  (bind _returnvalue_3 (Math|Conversions|ToLinearColor(Color) AltColour1))
  (bind (_r _g _b) (Math|Color|BreakColor _returnvalue))
  (bind (_r_2 _g_2 _b_2) (Math|Color|BreakColor _returnvalue_2))
  (bind (_r_3 _g_3 _b_3) (Math|Color|BreakColor _returnvalue_3))
  (for _array_element (Components|GetChildrenComponents Root true)
    (bind _asstatic_mesh_component (Utilities|Casting|CastToStaticMeshComponent _array_element))
    ;[1 1 1] Reset windows to blank walls
    (if (Utilities|String|Contains (Utilities|GetDisplayName _asstatic_mesh_component) "wall_window")
      (Components|StaticMesh|SetStaticMesh _asstatic_mesh_component "/Game/meshes/enviroment_assets/wall_blank.wall_blank"))
    ;[1 1 1] Chance on setting the wall as a window
    (if (Utilities|String|Contains (Utilities|GetDisplayName _asstatic_mesh_component) "wall_blank")
      (if (<= (Math|Random|RandomFloat) windowSpawnChance_)
        (Components|StaticMesh|SetStaticMesh _asstatic_mesh_component "/Game/meshes/enviroment_assets/wall_window.wall_window")
        ;[1 1 1] Lit/unlit chance
        (if (<= (Math|Random|RandomFloat) litWindowChance_)
          (Rendering|Material|SetMaterial _asstatic_mesh_component 2 "/Game/Materials/MI_window_emissive.MI_window_emissive")
          ;[1 1 1] Choice between main colour and alts
          (if (< (Math|Random|RandomFloat) uniqueWindowChance)
            (switch int (Math|Random|RandomInteger 2)
              (:0
                (Rendering|Material|SetVectorParameterValueonMaterials _asstatic_mesh_component "Emissive_colour" (Math|Vector|MakeVector _r_3 _g_3 _b_3)))
              (:1
                (Rendering|Material|SetVectorParameterValueonMaterials _asstatic_mesh_component "Emissive_colour" (Math|Vector|MakeVector _r_2 _g_2 _b_2))))
            (else
              (Rendering|Material|SetVectorParameterValueonMaterials _asstatic_mesh_component "Emissive_colour" (Math|Vector|MakeVector _r _g _b))))
          (else
            (Rendering|Material|SetMaterial _asstatic_mesh_component 2 "/Game/Materials/MI_window_emissive_off.MI_window_emissive_off")))))))