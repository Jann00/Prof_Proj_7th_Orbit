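; House blueprint for an environment building that randomises its windows when play begins.
; BeginPlay finds a BP_house_l06_02 actor in the level and calls its SpawnRandomWindows, passing this house's chances, colours and SharedRoot.
; An unconnected older graph holds local logic that swaps wall meshes by component name and randomly picks lit or unlit window materials.
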(event EventBeginPlay
  (bind _returnvalue (Actor|GetActorOfClass "/Game/meshes/enviroment_assets/assembled_components/BP_house_l06_02.BP_house_l06_02_C"))
  (Default|SpawnRandomWindows _returnvalue (Variables|Default|GetwindowSpawnChance) (Variables|Default|GetlitWindowChance) (Variables|Default|GetUniqueWindowChance) (Variables|Default|GetMainColour) (Variables|Default|GetAltColour1) (Variables|Default|GetAltColour2) (Variables|Default|GetSharedRoot)))

(event Collision|EventActorBeginOverlap
  (params (OtherActor :type Actor%20Object%20Reference)))

(event EventTick
  (params (DeltaSeconds :type Float%20%28single-precision%29)))

(fn ConstructionScript)